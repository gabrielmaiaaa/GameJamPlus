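; BP_Tiles is a grid tile actor that holds a Coordinate (row, column, ID, location) and places itself relative to its owner.
; The construction script writes those coordinate values to a TextRender label.
; Initialize snaps the tile onto a valid owner, then sets its relative location from CalculateLocation, which spaces tiles along negative X and Y by column and row using the Tile component's bounds.
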(event `self.ReceiveBeginPlay`)

(fn `CalculateLocation`
  (returns (OutLocation :type "Vector Structure"))
  (bind (_coordinate_row _coordinate_column) (break `/Game/Grid/StrGridCoordinate` (`self.Coordinate`)))
  (return (`KismetMathLibrary.MakeVector` (* (* _coordinate_column -2) (.x (`.BoxExtent` (`KismetSystemLibrary.GetComponentBounds` (`self.Tile`))))) (* (* _coordinate_row -2) (.y (`.BoxExtent` (`KismetSystemLibrary.GetComponentBounds` (`self.Tile`))))))))

(fn `Initialize`
  (bind _returnvalue (`self.GetOwner`))
  (`/Engine/EditorBlueprintResources/StandardMacros.IsValid` _returnvalue
    (:`Is Valid`
      (`self.K2_AttachToActor` _returnvalue "None" "SnapToTarget" "SnapToTarget" "KeepRelative" false)
      (bind _outlocation (`self.CalculateLocation`))
      (`self.K2_SetActorRelativeLocation` _outlocation))))

(fn `UserConstructionScript`
  (bind (_coordinate_row _coordinate_column _coordinate_id _coordinate_location) (break `/Game/Grid/StrGridCoordinate` (`self.Coordinate`)))
  (`TextRenderComponent.K2_SetText` (`self.TextRender`) (`KismetTextLibrary.Conv_StringToText` (`KismetStringLibrary.Concat_StrStr` "R:" (`KismetStringLibrary.Conv_IntToString` _coordinate_row) " \nC:" (`KismetStringLibrary.Conv_IntToString` _coordinate_column) " \nID:" (`KismetStringLibrary.Conv_IntToString` _coordinate_id) " \n" (`KismetStringLibrary.Conv_VectorToString` _coordinate_location)))))