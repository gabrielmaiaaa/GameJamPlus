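; Grid actor that builds a square, hexagon or triangle tile grid as instanced static meshes around its location.
; SpawnGrid pulls mesh data from DT_GridShapeData, snaps the center and derives each tile transform per shape, staggering hex tiles and flipping triangles.
; With UseEnvironment, debug-drawn sphere traces drop tiles lacking ground and snap the rest to height steps.
; The grid rebuilds on construction and again from Tick behind a one-second Delay.
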(event `self.ReceiveTick`
  (params (DeltaSeconds :type "Float (single-precision)"))
  (`KismetSystemLibrary.Delay` 1.0)
  (`self.SpawnGrid` (`self.K2_GetActorLocation`) (`self.GridTileSize`) (`self.GridTileCount`) (`self.GridShape`) true))

(fn `CalculateCenterAndBottomLeft`
  (returns (Center :type "Vector Structure") (BottomLeft :type "Vector Structure"))
  (locals (C :type "Vector Structure" :default (0.0 0.0 0.0)))
  (bind (_gridtilecount_x _gridtilecount_y) (break `IntPoint` (`self.GridTileCount`)))
  (switch `/Game/Blueprints/Core/Grid/GridShapes/Hexagon/E_GridShape` (`self.GridShape`)
    (:`NewEnumerator1`
      (set `local.C` (`/Game/Blueprints/Core/Utilities/BFL_Utilities.SnapVectorToVerctor` (`self.GridCenterLocation`) (`self.GridTileSize`)))
      (return (`local.C`) (- (`self.GridCenterLocation`) (`KismetMathLibrary.Conv_Vector2DToVector` (* (/ (- (`KismetMathLibrary.Conv_IntPointToVector2D` (`self.GridTileCount`)) (`KismetMathLibrary.MakeVector2D` (`KismetMathLibrary.SelectFloat` 0.0 1.0 (`/Game/Blueprints/Core/Utilities/BFL_Utilities.IsIntEvent` _gridtilecount_x)) (`KismetMathLibrary.SelectFloat` 0.0 1.0 (`/Game/Blueprints/Core/Utilities/BFL_Utilities.IsIntEvent` _gridtilecount_y)))) 2.0) (`KismetMathLibrary.Conv_VectorToVector2D` (`self.GridTileSize`)))))))
    (:`NewEnumerator2`
      (set `local.C` (`/Game/Blueprints/Core/Utilities/BFL_Utilities.SnapVectorToVerctor` (`self.GridCenterLocation`) (* (`self.GridTileSize`) (1.5 1.0 1.0))))
      (return (`local.C`) (- (`local.C`) (`/Game/Blueprints/Core/Utilities/BFL_Utilities.SnapVectorToVerctor` (* (`KismetMathLibrary.Conv_Vector2DToVector` (/ (`KismetMathLibrary.Conv_IntPointToVector2D` (`self.GridTileCount`)) (3.0 2.0))) (`self.GridTileSize`)) (* (`self.GridTileSize`) (1.5 1.0 1.0))))))
    (:`NewEnumerator3`
      (set `local.C` (`/Game/Blueprints/Core/Utilities/BFL_Utilities.SnapVectorToVerctor` (`self.GridCenterLocation`) (* (`self.GridTileSize`) (2.0 1.0 1.0))))
      (return (`local.C`) (- (`local.C`) (`/Game/Blueprints/Core/Utilities/BFL_Utilities.SnapVectorToVerctor` (`KismetMathLibrary.Conv_Vector2DToVector` (* (/ (- (`KismetMathLibrary.Conv_IntPointToVector2D` (`self.GridTileCount`)) (1.0 1.0)) (2.0 4.0)) (`KismetMathLibrary.Conv_VectorToVector2D` (`self.GridTileSize`)))) (* (`self.GridTileSize`) (2.0 1.0 1.0))))))))

(fn `DestroyGrid`
  (`InstancedStaticMeshComponent.ClearInstances` (`self.InstancedStaticMesh`)))

(fn `GetCurrentShapeData`
  (returns (ReturnValue :type "/Game/Blueprints/Core/Grid/GridShapes/S_GridShapeData Structure"))
  (bind _returnvalue (`|GetEnumeratorNameAsString` (`self.GridShape`)))
  (bind _returnvalue_2 (`|GetDataTableRow` "/Game/Blueprints/Core/Grid/GridShapes/DT_GridShapeData.DT_GridShapeData" (`KismetStringLibrary.Conv_StringToName` _returnvalue))
    (:`then`
      (return _returnvalue_2))
    (:`RowNotFound`
      (`KismetSystemLibrary.PrintString` (`KismetStringLibrary.Concat_StrStr` "Error- " _returnvalue) true true (struct :`R` 1.0 :`G` 0.012255 :`A` 1.0)))))

(fn `GetTileLocationFromGridIndex`
  (params (GridIndex :type "IntPoint Structure"))
  (returns (TileLocation :type "Vector Structure"))
  (return (+ (`self.GetBottomLeftCornerLocation`) (* (`self.GridTileSize`) (`KismetMathLibrary.Conv_Vector2DToVector` (* (`KismetMathLibrary.Conv_IntPointToVector2D` GridIndex) (select `/Game/Blueprints/Core/Grid/GridShapes/Hexagon/E_GridShape` (`self.GridShape`) :`NewEnumerator1` (1.0 1.0) :`NewEnumerator2` (0.75 0.5) :`NewEnumerator3` (1.0 0.5) :!type "Vector2D Structure")))))))

(fn `GetTileRotationFromGridIndex`
  (params (GridIndex :type "IntPoint Structure"))
  (returns (TileRotation :type "Rotator Structure"))
  (bind (_gridindex_x _gridindex_y) (break `IntPoint` (`local.GridIndex`)))
  (if (`|EnumEquality` (`self.GridShape`) "NewEnumerator3")
    (return (`KismetMathLibrary.MakeRotator` 0.0 0.0 (+ (`KismetMathLibrary.SelectFloat` 180.0 0.0 (`/Game/Blueprints/Core/Utilities/BFL_Utilities.IsIntEvent` _gridindex_x)) (`KismetMathLibrary.SelectFloat` 180.0 0.0 (`/Game/Blueprints/Core/Utilities/BFL_Utilities.IsIntEvent` _gridindex_y)))))
    (else
      (return))))

(fn `SpawnGrid`
  (params (CenterLocation :type "Vector Structure") (TileSize :type "Vector Structure") (TileCount :type "IntPoint Structure") (Shape :type "/Game/Blueprints/Core/Grid/GridShapes/Hexagon/E_GridShape Enum" :default "NewEnumerator0") (UseEnvironment :type Boolean))
  (locals (X :type Integer) (Y :type Integer) (TileTransform :type "Transform Structure") (Index :type "IntPoint Structure"))
  (bind (_gridtilecount_x _gridtilecount_y) (break `IntPoint` (`self.GridTileCount`)))
  (bind _instancedstaticmesh (`self.InstancedStaticMesh`))
  (bind (_tiletransform_location _tiletransform_rotation _tiletransform_scale) (`KismetMathLibrary.BreakTransform` (`local.TileTransform`)))
  (bind (_gridtilecount_x_2 _gridtilecount_y_2) (break `IntPoint` (`self.GridTileCount`)))
  (bind _gridtilecount_x_3 (break `IntPoint` (`self.GridTileCount`)))
  (bind (_meshsize _mesh _meshmaterial _flatmesh _flatbordermesh) (break `/Game/Blueprints/Core/Grid/GridShapes/S_GridShapeData` (`self.GetCurrentShapeData`)))
  (set `self.GridCenterLocation` CenterLocation)
  (set `self.GridTileSize` TileSize)
  (set `self.GridTileCount` TileCount)
  (set `self.GridShape` Shape)
  (`StaticMeshComponent.SetStaticMesh` _instancedstaticmesh _flatmesh)
  (`PrimitiveComponent.SetMaterial` _instancedstaticmesh 0 _flatbordermesh)
  (`self.DestroyGrid`)
  (bind (_center _bottomleft) (`self.CalculateCenterAndBottomLeft`))
  (set `self.GridCenterLocation` _center)
  (set `self.GetBottomLeftCornerLocation` _bottomleft)
  (for _index (range _gridtilecount_x_3)
    (set `local.X` _index)
    (if (`|EnumInequality` (`self.GridShape`) "NewEnumerator2")
      (for _index_2 (range _gridtilecount_y)
        (set `local.Y` _index_2)
        (set `local.Index` (make `IntPoint` (`local.X`) (`local.Y`)) :!label _label)
        (set `local.TileTransform` (`KismetMathLibrary.MakeTransform` (+ (`self.GetTileLocationFromGridIndex` (`local.Index`)) (0.0 0.0 2.0)) (`self.GetTileRotationFromGridIndex` (`local.Index`)) (/ (`self.GridTileSize`) (`.MeshSize_8_EDC71FE046C10D76C803A9870A028FC4` (break `/Game/Blueprints/Core/Grid/GridShapes/S_GridShapeData` (`self.GetCurrentShapeData`))))))
        (if (`local.UseEnvironment`)
          (bind (_hitsomething _outlocation) (`self.TraceForGround` _tiletransform_location))
          (if _hitsomething
            (set `local.TileTransform` (`KismetMathLibrary.MakeTransform` _outlocation _tiletransform_rotation _tiletransform_scale))
            (`InstancedStaticMeshComponent.AddInstanceWorldSpace` (`self.InstancedStaticMesh`) (`local.TileTransform`)))
          (else
            (`InstancedStaticMeshComponent.AddInstanceWorldSpace` (`self.InstancedStaticMesh`) (`local.TileTransform`)))))
      (else
        (for _index_3 (range (`KismetMathLibrary.SelectInt` 0 1 (`/Game/Blueprints/Core/Utilities/BFL_Utilities.IsIntEvent` (`local.X`))) (* _gridtilecount_y_2 2))
          (set `local.Y` _index_3)
          (`|ExecutionSequence`
            (:`then_0`
              (goto _label))
            (:`then_1`
              (`/Engine/EditorBlueprintResources/StandardMacros.IncrementInt` _index_3))))))))

(fn `TraceForGround`
  (params (Location :type "Vector Structure"))
  (returns (HitSomething :type Boolean) (OutLocation :type "Vector Structure"))
  (locals (Radius :type "Float (double-precision)" :default 0.0))
  (bind _location (`local.Location`))
  (bind _gridtilesize_x (`KismetMathLibrary.BreakVector` (`self.GridTileSize`)))
  (bind (_gridtilesize_x_2 _gridtilesize_y _gridtilesize_z) (`KismetMathLibrary.BreakVector` (`self.GridTileSize`)))
  (bind (_location_x _location_y) (`KismetMathLibrary.BreakVector` (`local.Location`)))
  (set `local.Radius` (/ _gridtilesize_x 3.0))
  (bind _outhits (`KismetSystemLibrary.SphereTraceMulti` :`Start` (+ _location (0.0 0.0 1000.0)) :`End` (- _location (0.0 0.0 1000.0)) :`Radius` (`local.Radius`) :`TraceChannel` "TraceTypeQuery3" :`DrawDebugType` "ForDuration"))
  (if (> (`KismetArrayLibrary.Array_Length` _outhits) 0)
    (return true (`KismetMathLibrary.MakeVector` _location_x _location_y (`KismetMathLibrary.GridSnap_Float` (.z (`.Location` (`GameplayStatics.BreakHitResult` (`|GetArrayItem` _outhits)))) _gridtilesize_z)))
    (else
      (return false (`local.Location`)))))

(fn `UserConstructionScript`
  (`self.SpawnGrid` (`self.K2_GetActorLocation`) (`self.GridTileSize`) (`self.GridTileCount`) (`self.GridShape`) true))