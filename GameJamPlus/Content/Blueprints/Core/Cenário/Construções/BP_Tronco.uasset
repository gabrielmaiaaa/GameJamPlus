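; BP_Tronco is a log (tronco) platform that moves in fixed steps along world X and carries the player.
; Overlap events on PlayerTouch track whether the Player is on it.
; Each AndarTronco call waits briefly, then shifts the Cube, plus the player's root when aboard.
; When the Cube's X exactly equals the end value, the actor destroys itself and spawns a replacement at its actor transform.
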(event `self.PlayerTouch.OnComponentEndOverlap`
  (params (OverlappedComponent :type "PrimitiveComponent Object Reference") (OtherActor :type "Actor Object Reference") (OtherComp :type "PrimitiveComponent Object Reference") (OtherBodyIndex :type Integer))
  (bind _asplayer (cast `/Game/Blueprints/Core/Player/Player2/Player` OtherActor))
  (set `self.As Player` _asplayer)
  (set `self.PlayerNoTronco` false))

(event `self.PlayerTouch.OnComponentBeginOverlap`
  (params (OverlappedComponent :type "PrimitiveComponent Object Reference") (OtherActor :type "Actor Object Reference") (OtherComp :type "PrimitiveComponent Object Reference") (OtherBodyIndex :type Integer) (bFromSweep :type Boolean) (SweepResult :type "HitResult Structure (by ref)"))
  (bind _asplayer (cast `/Game/Blueprints/Core/Player/Player2/Player` OtherActor))
  (set `self.As Player` _asplayer)
  (set `self.PlayerNoTronco` true))

(event `AndarTronco`
  (bind _cube (`self.Cube`))
  (bind _cube_2 (`self.Cube`))
  (bind _as_player (`self.As Player`))
  (bind (_returnvalue_x _returnvalue_y _returnvalue_z) (`KismetMathLibrary.BreakVector` (`SceneComponent.K2_GetComponentLocation` _cube)))
  (bind _returnvalue_x_2 (`KismetMathLibrary.BreakVector` (`SceneComponent.K2_GetComponentLocation` (`self.Cube`))))
  (bind _returnvalue_x_3 (`KismetMathLibrary.BreakVector` (`SceneComponent.K2_GetComponentLocation` (`self.Cube`))))
  (bind (_returnvalue_x_4 _returnvalue_y_2 _returnvalue_z_2) (`KismetMathLibrary.BreakVector` (`SceneComponent.K2_GetComponentLocation` _cube_2)))
  (bind (_returnvalue_x_5 _returnvalue_y_3 _returnvalue_z_3) (`KismetMathLibrary.BreakVector` (`SceneComponent.K2_GetComponentLocation` (`Actor.RootComponent` _as_player))))
  (`KismetSystemLibrary.Delay` 0.005)
  (if (`self.PlayerNoTronco`)
    (`SceneComponent.K2_SetWorldLocation` _cube_2 (`KismetMathLibrary.MakeVector` (+ _returnvalue_x_4 200.0) _returnvalue_y_2 _returnvalue_z_2) false false)
    (`SceneComponent.K2_SetWorldLocation` (`Actor.RootComponent` _as_player) (`KismetMathLibrary.MakeVector` (+ _returnvalue_x_5 200.0) _returnvalue_y_3 _returnvalue_z_3) false false)
    (if (== _returnvalue_x_3 1800.0)
      (`self.K2_DestroyActor`)
      (`|SpawnActorFromClass` "BP_Tronco_C" (`self.GetTransform`) "Undefined" "OverrideRootScale" null null))
    (else
      (`SceneComponent.K2_SetWorldLocation` _cube (`KismetMathLibrary.MakeVector` (+ _returnvalue_x 200.0) _returnvalue_y _returnvalue_z) false false)
      (if (== _returnvalue_x_2 1800.0)
        (`self.K2_DestroyActor`)
        (`|SpawnActorFromClass` "BP_Tronco_C" (`self.GetTransform`) "Undefined" "OverrideRootScale" null null)))))

(fn `UserConstructionScript`)