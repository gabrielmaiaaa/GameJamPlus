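; BP_Tronco is a scenery log actor ("tronco") that moves along world X and replaces itself at an end point.
; Each AndarTronco call waits briefly, then shifts the Cube component one fixed step along X, with nothing in this graph repeating the call.
; When Cube's X exactly equals the limit, the actor destroys itself and spawns a new BP_Tronco at the actor's transform.
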(event `AndarTronco`
  (bind _cube (`self.Cube`))
  (bind _returnvalue_x (`KismetMathLibrary.BreakVector` (`SceneComponent.K2_GetComponentLocation` (`self.Cube`))))
  (bind (_returnvalue_x_2 _returnvalue_y _returnvalue_z) (`KismetMathLibrary.BreakVector` (`SceneComponent.K2_GetComponentLocation` _cube)))
  (`KismetSystemLibrary.Delay` 0.005)
  (`SceneComponent.K2_SetWorldLocation` _cube (`KismetMathLibrary.MakeVector` (+ _returnvalue_x_2 200.0) _returnvalue_y _returnvalue_z) false false)
  (if (== _returnvalue_x 2000.0)
    (`self.K2_DestroyActor`)
    (`|SpawnActorFromClass` "BP_Tronco_C" (`self.GetTransform`) "Undefined" "OverrideRootScale" null null)))

(fn `UserConstructionScript`)