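; Grid-walking animal (pig, "Porco") that roams BP_Generator's tile map on its own, starting southward from its ID tile.
; North, East, South and West events each repeat their heading after a delay, turning clockwise at map edges or tiles listed in IDError.
; North/South step by one ID with an X-spacing check against row wrap; East/West step by column count.
; Timelines lerp XY movement while updating grid tiles and neighbours.
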(event `self.ReceiveBeginPlay`
  (bind _returnvalue (`GameplayStatics.GetActorOfClass` "/Game/Grid/BP_Generator.BP_Generator_C"))
  (bind _output_get (set `self.Grid` _returnvalue))
  (set `self.Neightbors` (`/Game/Grid/BP_Generator.GetTileNeightbors` _output_get (`self.ID`) false))
  (`self.K2_SetActorLocation` (`/Game/Grid/BP_Generator.GetTileLocation` _output_get (`self.ID`)))
  (`self.South`))

(event `North`
  (bind (_returnvalue_x _returnvalue_y _returnvalue_z) (`KismetMathLibrary.BreakVector` (`self.K2_GetActorLocation`)))
  (bind _id (`self.ID`))
  (bind _returnvalue (- (`self.ID`) 1))
  (bind (_outlocation_x _outlocation_y) (`KismetMathLibrary.BreakVector` (`/Game/Grid/BP_Generator.GetNeightborLocation` (`self.Grid`) (`self.Neightbors`) (`self.NewID`))))
  (bind _returnvalue_2 (+ _id 1))
  (bind _tiles (`/Game/Grid/BP_Generator.Tiles` (`self.Grid`)))
  (bind _tiles_2 (`/Game/Grid/BP_Generator.Tiles` (`self.Grid`)))
  (bind _liberado (`self.VerrificaErro` _returnvalue_2))
  (if _liberado
    (if (< _id (`/Game/Grid/BP_Generator.GetMaxID` (`self.Grid`)))
      (if (== (- (.x (`.Location_11_1437950641631F2A1BD6EBA6314F3D6D` (break `/Game/Grid/StrGridCoordinate` (`/Game/Grid/BP_Tiles.Coordinate` (`|GetArrayItem` _tiles_2 _id))))) (.x (`.Location_11_1437950641631F2A1BD6EBA6314F3D6D` (break `/Game/Grid/StrGridCoordinate` (`/Game/Grid/BP_Tiles.Coordinate` (`|GetArrayItem` _tiles_2 _returnvalue_2)))))) -100.0)
        (set `self.NewID` _returnvalue_2)
        (bind (_direction _movealpha) (`Timeline|Timeline_1` :!via `PlayFromStart`)
          (:`Update`
            (`self.K2_SetActorLocation` (`KismetMathLibrary.VLerp` (`KismetMathLibrary.MakeVector` _returnvalue_x _returnvalue_y _returnvalue_z) (`KismetMathLibrary.MakeVector` _outlocation_x _outlocation_y _returnvalue_z) _movealpha))
            (`/Game/Grid/BP_Generator.UpdateTilesPorco` (`self.Grid`) (`|GetArrayItem` _tiles (`self.NewID`)) (`self.NewID`) _returnvalue (`|GetArrayItem` _tiles _returnvalue))
            (bind _output_get (set `self.ID` (`self.NewID`)))
            (set `self.Neightbors` (`/Game/Grid/BP_Generator.GetTileNeightbors` (`self.Grid`) _output_get false))
            (`KismetSystemLibrary.Delay` 1.0)
            (`self.North`)))
        (else
          (`self.East`)))
      (else
        (`self.East` :!label _label)))
    (else
      (goto _label))))

(event `East`
  (bind (_returnvalue_x _returnvalue_y _returnvalue_z) (`KismetMathLibrary.BreakVector` (`self.K2_GetActorLocation`)))
  (bind (_outlocation_x _outlocation_y) (`KismetMathLibrary.BreakVector` (`/Game/Grid/BP_Generator.GetNeightborLocation` (`self.Grid`) (`self.Neightbors`) (`self.NewID`))))
  (bind _tiles (`/Game/Grid/BP_Generator.Tiles` (`self.Grid`)))
  (bind (_mapsize_row _mapsize_column) (break `/Game/Grid/StrGridCoordinate` (`/Game/Grid/BP_Generator.MapSize` (`self.Grid`))))
  (bind (_mapsize_row_2 _mapsize_column_2) (break `/Game/Grid/StrGridCoordinate` (`/Game/Grid/BP_Generator.MapSize` (`self.Grid`))))
  (bind _returnvalue (- (`self.ID`) _mapsize_column))
  (bind _returnvalue_2 (+ (`self.ID`) _mapsize_column_2))
  (bind _liberado (`self.VerrificaErro` _returnvalue_2))
  (if _liberado
    (if (< _returnvalue_2 (`/Game/Grid/BP_Generator.GetMaxID` (`self.Grid`)))
      (set `self.NewId` _returnvalue_2)
      (bind (_direction _movealpha) (`Timeline|Timeline_2` :!via `PlayFromStart`)
        (:`Update`
          (`self.K2_SetActorLocation` (`KismetMathLibrary.VLerp` (`KismetMathLibrary.MakeVector` _returnvalue_x _returnvalue_y _returnvalue_z) (`KismetMathLibrary.MakeVector` _outlocation_x _outlocation_y _returnvalue_z) _movealpha))
          (`/Game/Grid/BP_Generator.UpdateTilesPorco` (`self.Grid`) (`|GetArrayItem` _tiles (`self.NewID`)) (`self.NewID`) _returnvalue (`|GetArrayItem` _tiles _returnvalue))
          (bind _output_get (set `self.ID` (`self.NewId`)))
          (set `self.Neightbors` (`/Game/Grid/BP_Generator.GetTileNeightbors` (`self.Grid`) _output_get false))
          (`KismetSystemLibrary.Delay` 1.0)
          (`self.East`)))
      (else
        (`self.South` :!label _label_2)))
    (else
      (goto _label_2))))

(event `South`
  (bind (_returnvalue_x _returnvalue_y _returnvalue_z) (`KismetMathLibrary.BreakVector` (`self.K2_GetActorLocation`)))
  (bind _id (`self.ID`))
  (bind _returnvalue (- _id 1))
  (bind (_outlocation_x _outlocation_y) (`KismetMathLibrary.BreakVector` (`/Game/Grid/BP_Generator.GetNeightborLocation` (`self.Grid`) (`self.Neightbors`) (`self.NewID`))))
  (bind _returnvalue_2 (+ (`self.ID`) 1))
  (bind _tiles (`/Game/Grid/BP_Generator.Tiles` (`self.Grid`)))
  (bind _tiles_2 (`/Game/Grid/BP_Generator.Tiles` (`self.Grid`)))
  (bind _liberado (`self.VerrificaErro` _returnvalue))
  (if _liberado
    (if (> _returnvalue -1)
      (if (== (- (.x (`.Location_11_1437950641631F2A1BD6EBA6314F3D6D` (break `/Game/Grid/StrGridCoordinate` (`/Game/Grid/BP_Tiles.Coordinate` (`|GetArrayItem` _tiles_2 _returnvalue))))) (.x (`.Location_11_1437950641631F2A1BD6EBA6314F3D6D` (break `/Game/Grid/StrGridCoordinate` (`/Game/Grid/BP_Tiles.Coordinate` (`|GetArrayItem` _tiles_2 _id)))))) -100.0)
        (set `self.NewID` _returnvalue)
        (bind (_direction _movealpha) (`Timeline|Timeline_0` :!via `PlayFromStart`)
          (:`Update`
            (`self.K2_SetActorLocation` (`KismetMathLibrary.VLerp` (`KismetMathLibrary.MakeVector` _returnvalue_x _returnvalue_y _returnvalue_z) (`KismetMathLibrary.MakeVector` _outlocation_x _outlocation_y _returnvalue_z) _movealpha))
            (`/Game/Grid/BP_Generator.UpdateTilesPorco` (`self.Grid`) (`|GetArrayItem` _tiles (`self.NewID`)) (`self.NewID`) _returnvalue_2 (`|GetArrayItem` _tiles _returnvalue_2))
            (bind _output_get (set `self.ID` (`self.NewID`)))
            (set `self.Neightbors` (`/Game/Grid/BP_Generator.GetTileNeightbors` (`self.Grid`) _output_get false))
            (`KismetSystemLibrary.Delay` 1.0)
            (`self.South`)))
        (else
          (`self.West`)))
      (else
        (`self.West` :!label _label_3)))
    (else
      (goto _label_3))))

(event `West`
  (bind (_returnvalue_x _returnvalue_y _returnvalue_z) (`KismetMathLibrary.BreakVector` (`self.K2_GetActorLocation`)))
  (bind (_outlocation_x _outlocation_y) (`KismetMathLibrary.BreakVector` (`/Game/Grid/BP_Generator.GetNeightborLocation` (`self.Grid`) (`self.Neightbors`) (`self.NewID`))))
  (bind (_mapsize_row _mapsize_column) (break `/Game/Grid/StrGridCoordinate` (`/Game/Grid/BP_Generator.MapSize` (`self.Grid`))))
  (bind _tiles (`/Game/Grid/BP_Generator.Tiles` (`self.Grid`)))
  (bind (_mapsize_row_2 _mapsize_column_2) (break `/Game/Grid/StrGridCoordinate` (`/Game/Grid/BP_Generator.MapSize` (`self.Grid`))))
  (bind _returnvalue (- (`self.ID`) _mapsize_column))
  (bind _returnvalue_2 (+ (`self.ID`) _mapsize_column_2))
  (bind _liberado (`self.VerrificaErro` _returnvalue))
  (if _liberado
    (if (> _returnvalue -1)
      (set `self.NewId` _returnvalue)
      (bind (_direction _movealpha) (`Timeline|Timeline_3` :!via `PlayFromStart`)
        (:`Update`
          (`self.K2_SetActorLocation` (`KismetMathLibrary.VLerp` (`KismetMathLibrary.MakeVector` _returnvalue_x _returnvalue_y _returnvalue_z) (`KismetMathLibrary.MakeVector` _outlocation_x _outlocation_y _returnvalue_z) _movealpha))
          (`/Game/Grid/BP_Generator.UpdateTilesPorco` (`self.Grid`) (`|GetArrayItem` _tiles (`self.NewID`)) (`self.NewID`) _returnvalue_2 (`|GetArrayItem` _tiles _returnvalue_2))
          (bind _output_get (set `self.ID` (`self.NewId`)))
          (set `self.Neightbors` (`/Game/Grid/BP_Generator.GetTileNeightbors` (`self.Grid`) _output_get false))
          (`KismetSystemLibrary.Delay` 1.0)
          (`self.West`)))
      (else
        (`self.North` :!label _label_4)))
    (else
      (goto _label_4))))

(fn `UserConstructionScript`)

(fn `VerrificaErro`
  (params (ID :type Integer))
  (returns (Liberado :type Boolean))
  (for _array_element (`/Game/Grid/BP_Generator.IDError` (`self.Grid`))
    (if (== _array_element ID)
      (return false)))
  (return true))