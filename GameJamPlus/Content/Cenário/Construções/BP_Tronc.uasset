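; BP_Tronc is a moving log on the BP_Generator tile grid that tracks whether BP_Player is on it through a box overlap.
; Every two seconds TroncoAndaPai steps to tile ID-1, updating the grid and the riding player's tile ID, with a timeline lerp for movement.
; When that tile is not 100 units back in X, it resets any rider to their initial tile, destroys itself and spawns a replacement.
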(event `self.ReceiveBeginPlay`
  (bind (_returnvalue_x _returnvalue_y _returnvalue_z) (`KismetMathLibrary.BreakVector` (`self.K2_GetActorLocation`)))
  (bind _returnvalue (`GameplayStatics.GetActorOfClass` "/Game/Grid/BP_Generator.BP_Generator_C"))
  (bind _output_get (set `self.Grid` _returnvalue))
  (for _array_element (`/Game/Grid/BP_Generator.GetTileNeightbors` _returnvalue (`self.ID`) false)
    (`KismetArrayLibrary.Array_Add` (`self.Vizinhos`) _array_element))
  (bind (_outlocation_x _outlocation_y) (`KismetMathLibrary.BreakVector` (`/Game/Grid/BP_Generator.GetTileLocation` _output_get (`self.ID`))))
  (`self.K2_SetActorLocation` (`KismetMathLibrary.MakeVector` _outlocation_x _outlocation_y _returnvalue_z))
  (`KismetSystemLibrary.Delay` 2.0)
  (`self.TroncoAndaPai`))

(event `TroncoAndaPai`
  (bind (_returnvalue_x _returnvalue_y _returnvalue_z) (`KismetMathLibrary.BreakVector` (`self.K2_GetActorLocation`)))
  (bind _id (`self.ID`))
  (bind _id_2 (`self.ID`))
  (bind _as_bp_player (`self.As BP Player`))
  (bind _as_bp_player_2 (`self.As BP Player`))
  (bind _grid (`self.Grid`))
  (bind _grid_2 (`self.Grid`))
  (bind (_outlocation_x _outlocation_y) (`KismetMathLibrary.BreakVector` (`/Game/Grid/BP_Generator.GetNeightborLocation` (`self.Grid`) (`self.Vizinhos`) (`self.NewId`))))
  (bind _returnvalue (- (`self.ID`) 1))
  (bind _idinicial (`/Game/Player/BP_Player.IDInicial` _as_bp_player))
  (bind _tiles (`/Game/Grid/BP_Generator.Tiles` (`self.Grid`)))
  (bind _output (`|GetArrayItem` (`/Game/Grid/BP_Generator.Tiles` _grid) _id_2))
  (bind (_coordinate_row _coordinate_column _coordinate_id _coordinate_location) (break `/Game/Grid/StrGridCoordinate` (`/Game/Grid/BP_Tiles.Coordinate` _output)))
  (if (== (- (.x (`.Location_11_1437950641631F2A1BD6EBA6314F3D6D` (break `/Game/Grid/StrGridCoordinate` (`/Game/Grid/BP_Tiles.Coordinate` (`|GetArrayItem` _tiles _returnvalue))))) (.x (`.Location_11_1437950641631F2A1BD6EBA6314F3D6D` (break `/Game/Grid/StrGridCoordinate` (`/Game/Grid/BP_Tiles.Coordinate` (`|GetArrayItem` _tiles (`self.ID`))))))) -100.0)
    (if (`self.PlayerDentro`)
      (bind _output_get (set `/Game/Player/BP_Player.ID` _returnvalue (`self.As BP Player`)))
      (`/Game/Player/BP_Player.ResetaVizinhos` (`self.As BP Player`) _output_get))
    (`/Game/Grid/BP_Generator.UpdateTilesTronco` _grid _coordinate_location _output _id_2 _returnvalue true)
    (set `self.NewId` _returnvalue)
    (bind (_direction _movealpha) (`Timeline|Timeline_0` :!via `PlayFromStart`)
      (:`Update`
        (`self.K2_SetActorLocation` (`KismetMathLibrary.VLerp` (`KismetMathLibrary.MakeVector` _returnvalue_x _returnvalue_y _returnvalue_z) (`KismetMathLibrary.MakeVector` _outlocation_x _outlocation_y _returnvalue_z) _movealpha))
        (bind _output_get_2 (set `self.ID` (`self.NewId`)))
        (set `self.Vizinhos` (`/Game/Grid/BP_Generator.GetTileNeightbors` (`self.Grid`) _output_get_2 false))
        (`KismetSystemLibrary.Delay` 2.0)
        (`self.TroncoAndaPai`)))
    (else
      (if (`self.PlayerDentro`)
        (bind _output_get_3 (set `/Game/Player/BP_Player.ID` _idinicial _as_bp_player))
        (`/Game/Player/BP_Player.ResetaVizinhos` _as_bp_player_2 _idinicial)
        (`self.K2_SetActorLocation` _as_bp_player_2 (`/Game/Grid/BP_Generator.GetTileLocation` (`self.Grid`) _output_get_3) false false))
      (`self.K2_DestroyActor`)
      (`|SpawnActorFromClass` "BP_Tronc_C" (`self.GetTransform`) "Undefined" "OverrideRootScale" null null)
      (`/Game/Grid/BP_Generator.UpdateTilesTronco` _grid_2 (0.0 0.0 0.0) (`|GetArrayItem` (`/Game/Grid/BP_Generator.Tiles` _grid_2) _id) _id 0 false))))

(event `self.Box.OnComponentBeginOverlap`
  (params (OverlappedComponent :type "PrimitiveComponent Object Reference") (OtherActor :type "Actor Object Reference") (OtherComp :type "PrimitiveComponent Object Reference") (OtherBodyIndex :type Integer) (bFromSweep :type Boolean) (SweepResult :type "HitResult Structure (by ref)"))
  (bind _asbp_player (cast `/Game/Player/BP_Player` OtherActor))
  (set `self.As BP Player` _asbp_player)
  (set `self.PlayerDentro` true))

(event `self.Box.OnComponentEndOverlap`
  (params (OverlappedComponent :type "PrimitiveComponent Object Reference") (OtherActor :type "Actor Object Reference") (OtherComp :type "PrimitiveComponent Object Reference") (OtherBodyIndex :type Integer))
  (bind _asbp_player (cast `/Game/Player/BP_Player` OtherActor))
  (set `self.As BP Player` _asbp_player)
  (set `self.PlayerDentro` false))

(fn `UserConstructionScript`)

(fn `VerificaErro`
  (params (ID :type Integer))
  (returns (Liberado :type Boolean))
  (for _array_element (`/Game/Grid/BP_Generator.IDError` (`self.Grid`))
    (if (== _array_element ID)
      (return false)))
  (return true))