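; Player actor that steps tile by tile across the BP_Generator grid and controls camera zoom.
; Axis inputs offset the tile ID by one or the column count, rejecting IDError tiles, out-of-range IDs and row wraps.
; Timelines lerp the actor to the neighbour tile, with DoOnce gates and delayed resets throttling steps.
; Zoom input drives BP_PosicaoCamera's interpolated spring arm length and offsets the camera from that actor each Tick.
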(event `self.ReceiveBeginPlay`
  (bind _returnvalue (`GameplayStatics.GetActorOfClass` "/Game/Player/BP_PosicaoCamera.BP_PosicaoCamera_C"))
  (set `self.PosicaoCamera` _returnvalue)
  (set `self.Zoom_Desired` (`SpringArmComponent.TargetArmLength` (`self.GetComponentByClass` (`self.PosicaoCamera`) "/Script/Engine.SpringArmComponent")))
  (bind _returnvalue_2 (`GameplayStatics.GetActorOfClass` "/Game/Grid/BP_Generator.BP_Generator_C"))
  (bind _output_get (set `self.Grid` _returnvalue_2))
  (for _array_element (`/Game/Grid/BP_Generator.GetTileNeightbors` _returnvalue_2 (`self.ID`) false)
    (`KismetArrayLibrary.Array_Add` (`self.Vizinhos`) _array_element))
  (`self.K2_SetActorLocation` (`/Game/Grid/BP_Generator.GetTileLocation` _output_get (`self.ID`))))

(event `self.ReceiveTick`
  (params (DeltaSeconds :type "Float (single-precision)"))
  (bind _position (`self.Position`))
  (bind _returnvalue (`self.GetComponentByClass` (`self.PosicaoCamera`) "/Script/Engine.SpringArmComponent"))
  (bind (_returnvalue_x _returnvalue_y _returnvalue_z) (`KismetMathLibrary.BreakVector` (`SceneComponent.K2_GetComponentLocation` (`Actor.RootComponent` (`self.PosicaoCamera`)))))
  (`SceneComponent.K2_SetWorldLocation` (`self.Camera`) (`KismetMathLibrary.MakeVector` (+ _returnvalue_x _position) _returnvalue_y (- _returnvalue_z (/ _position 2.0))) false false)
  (set `SpringArmComponent.TargetArmLength` (`KismetMathLibrary.FInterpTo` (`SpringArmComponent.TargetArmLength` _returnvalue) (`self.Zoom_Desired`) DeltaSeconds) _returnvalue))

(event `InputAxis|InputAxios_Zoom`
  (params (AxisValue :type "Float (single-precision)"))
  (bind _output_get (set `self.Zoom_Desired` (`KismetMathLibrary.FClamp` (+ (* AxisValue -40.0) (`self.Zoom_Desired`)) 750.0 1250.0)))
  (set `self.Position` _output_get))

(event `InputAxis|InputAxios_Forward`
  (params (AxisValue :type "Float (single-precision)"))
  (bind (_returnvalue_x _returnvalue_y _returnvalue_z) (`KismetMathLibrary.BreakVector` (`self.K2_GetActorLocation`)))
  (bind (_returnvalue_x_2 _returnvalue_y_2 _returnvalue_z_2) (`KismetMathLibrary.BreakVector` (`self.K2_GetActorLocation`)))
  (bind _id (`self.ID`))
  (bind _returnvalue (- _id 1))
  (bind _returnvalue_2 (+ (`self.ID`) 1))
  (bind _tiles (`/Game/Grid/BP_Generator.Tiles` (`self.Grid`)))
  (bind _tiles_2 (`/Game/Grid/BP_Generator.Tiles` (`self.Grid`)))
  (if (== AxisValue -1.0)
    (`/Engine/EditorBlueprintResources/StandardMacros.DoOnce` false :!label _label
      (:`Completed`
        (bind _liberado (`self.VerificaError` _returnvalue))
        (if _liberado
          (if (> _returnvalue -1)
            (if (== (- (.x (`.Location_11_1437950641631F2A1BD6EBA6314F3D6D` (break `/Game/Grid/StrGridCoordinate` (`/Game/Grid/BP_Tiles.Coordinate` (`|GetArrayItem` _tiles_2 _returnvalue))))) (.x (`.Location_11_1437950641631F2A1BD6EBA6314F3D6D` (break `/Game/Grid/StrGridCoordinate` (`/Game/Grid/BP_Tiles.Coordinate` (`|GetArrayItem` _tiles_2 _id)))))) -100.0)
              (set `self.NewId` _returnvalue)
              (bind _returnvalue_3 (`GameplayStatics.GetActorOfClass` "/Game/Grid/BP_Generator.BP_Generator_C"))
              (bind (_direction _movealpha) (`Timeline|Timeline_0` :!via `PlayFromStart`)
                (:`Update`
                  (bind (_outlocation_x _outlocation_y _outlocation_z) (`KismetMathLibrary.BreakVector` (`/Game/Grid/BP_Generator.GetNeightborLocation` _returnvalue_3 (`self.Vizinhos`) (`self.NewId`))))
                  (`self.K2_SetActorLocation` (`KismetMathLibrary.VLerp` (`KismetMathLibrary.MakeVector` _returnvalue_x _returnvalue_y _returnvalue_z) (`KismetMathLibrary.MakeVector` _outlocation_x _outlocation_y (+ _outlocation_z 89.0)) _movealpha))
                  (bind _output_get (set `self.ID` (`self.NewId`)))
                  (set `self.Vizinhos` (`/Game/Grid/BP_Generator.GetTileNeightbors` _returnvalue_3 _output_get false))
                  (`KismetSystemLibrary.Delay` 0.5)
                  (`self.Reset`)))
              (else
                (`self.Reset`)))
            (else
              (`self.Reset` :!label _label_2)))
          (else
            (goto _label_2)))))
    (elif (== AxisValue 1.0)
      (`/Engine/EditorBlueprintResources/StandardMacros.DoOnce` false :!label _label_3
        (:`Completed`
          (bind _liberado_2 (`self.VerificaError` _returnvalue_2))
          (if _liberado_2
            (if (< _returnvalue_2 (`/Game/Grid/BP_Generator.GetMaxID` (`self.Grid`)))
              (if (== (- (.x (`.Location_11_1437950641631F2A1BD6EBA6314F3D6D` (break `/Game/Grid/StrGridCoordinate` (`/Game/Grid/BP_Tiles.Coordinate` (`|GetArrayItem` _tiles (`self.ID`)))))) (.x (`.Location_11_1437950641631F2A1BD6EBA6314F3D6D` (break `/Game/Grid/StrGridCoordinate` (`/Game/Grid/BP_Tiles.Coordinate` (`|GetArrayItem` _tiles _returnvalue_2)))))) -100.0)
                (set `self.NewId` _returnvalue_2)
                (bind _returnvalue_4 (`GameplayStatics.GetActorOfClass` "/Game/Grid/BP_Generator.BP_Generator_C"))
                (bind (_direction_2 _movealpha_2) (`Timeline|Timeline_1` :!via `PlayFromStart`)
                  (:`Update`
                    (bind (_outlocation_x_2 _outlocation_y_2 _outlocation_z_2) (`KismetMathLibrary.BreakVector` (`/Game/Grid/BP_Generator.GetNeightborLocation` _returnvalue_4 (`self.Vizinhos`) (`self.NewId`))))
                    (`self.K2_SetActorLocation` (`KismetMathLibrary.VLerp` (`KismetMathLibrary.MakeVector` _returnvalue_x_2 _returnvalue_y_2 _returnvalue_z_2) (`KismetMathLibrary.MakeVector` _outlocation_x_2 _outlocation_y_2 (+ _outlocation_z_2 89.0)) _movealpha_2))
                    (bind _output_get_2 (set `self.ID` (`self.NewId`)))
                    (set `self.Vizinhos` (`/Game/Grid/BP_Generator.GetTileNeightbors` _returnvalue_4 _output_get_2 false))
                    (`KismetSystemLibrary.Delay` 0.5)
                    (`self.Reset2`)))
                (else
                  (`self.Reset2`)))
              (else
                (`self.Reset2` :!label _label_4)))
            (else
              (goto _label_4))))))))

(event `Reset`
  (goto _label :!via `Reset`))

(event `Reset2`
  (goto _label_3 :!via `Reset`))

(event `InputAxis|inputAxios_Right`
  (params (AxisValue :type "Float (single-precision)"))
  (bind (_returnvalue_x _returnvalue_y _returnvalue_z) (`KismetMathLibrary.BreakVector` (`self.K2_GetActorLocation`)))
  (bind (_returnvalue_x_2 _returnvalue_y_2 _returnvalue_z_2) (`KismetMathLibrary.BreakVector` (`self.K2_GetActorLocation`)))
  (bind (_mapsize_row _mapsize_column) (break `/Game/Grid/StrGridCoordinate` (`/Game/Grid/BP_Generator.MapSize` (`self.Grid`))))
  (bind (_mapsize_row_2 _mapsize_column_2) (break `/Game/Grid/StrGridCoordinate` (`/Game/Grid/BP_Generator.MapSize` (`self.Grid`))))
  (bind _returnvalue (- (`self.ID`) _mapsize_column_2))
  (bind _returnvalue_2 (+ (`self.ID`) _mapsize_column))
  (if (== AxisValue -1.0)
    (`/Engine/EditorBlueprintResources/StandardMacros.DoOnce` false :!label _label_5
      (:`Completed`
        (bind _liberado (`self.VerificaError` _returnvalue))
        (if _liberado
          (if (> _returnvalue -1)
            (set `self.NewId` _returnvalue)
            (bind _returnvalue_3 (`GameplayStatics.GetActorOfClass` "/Game/Grid/BP_Generator.BP_Generator_C"))
            (bind (_direction _movealpha) (`Timeline|Timeline_2` :!via `PlayFromStart`)
              (:`Update`
                (bind (_outlocation_x _outlocation_y _outlocation_z) (`KismetMathLibrary.BreakVector` (`/Game/Grid/BP_Generator.GetNeightborLocation` _returnvalue_3 (`self.Vizinhos`) (`self.NewId`))))
                (`self.K2_SetActorLocation` (`KismetMathLibrary.VLerp` (`KismetMathLibrary.MakeVector` _returnvalue_x_2 _returnvalue_y_2 _returnvalue_z_2) (`KismetMathLibrary.MakeVector` _outlocation_x _outlocation_y (+ _outlocation_z 89.0)) _movealpha))
                (bind _output_get (set `self.ID` (`self.NewId`)))
                (set `self.Vizinhos` (`/Game/Grid/BP_Generator.GetTileNeightbors` _returnvalue_3 _output_get false))
                (`KismetSystemLibrary.Delay` 0.5)
                (`self.Reset3`)))
            (else
              (`self.Reset3` :!label _label_6)))
          (else
            (goto _label_6)))))
    (elif (== AxisValue 1.0)
      (`/Engine/EditorBlueprintResources/StandardMacros.DoOnce` false :!label _label_7
        (:`Completed`
          (bind _liberado_2 (`self.VerificaError` _returnvalue_2))
          (if _liberado_2
            (if (< _returnvalue_2 (`/Game/Grid/BP_Generator.GetMaxID` (`self.Grid`)))
              (set `self.NewId` _returnvalue_2)
              (bind _returnvalue_4 (`GameplayStatics.GetActorOfClass` "/Game/Grid/BP_Generator.BP_Generator_C"))
              (bind (_direction_2 _movealpha_2) (`Timeline|Timeline_3` :!via `PlayFromStart`)
                (:`Update`
                  (bind (_outlocation_x_2 _outlocation_y_2 _outlocation_z_2) (`KismetMathLibrary.BreakVector` (`/Game/Grid/BP_Generator.GetNeightborLocation` _returnvalue_4 (`self.Vizinhos`) (`self.NewId`))))
                  (`self.K2_SetActorLocation` (`KismetMathLibrary.VLerp` (`KismetMathLibrary.MakeVector` _returnvalue_x _returnvalue_y _returnvalue_z) (`KismetMathLibrary.MakeVector` _outlocation_x_2 _outlocation_y_2 (+ _outlocation_z_2 89.0)) _movealpha_2))
                  (bind _output_get_2 (set `self.ID` (`self.NewId`)))
                  (set `self.Vizinhos` (`/Game/Grid/BP_Generator.GetTileNeightbors` _returnvalue_4 _output_get_2 false))
                  (`KismetSystemLibrary.Delay` 0.5)
                  (`self.Reset4`)))
              (else
                (`self.Reset4` :!label _label_8)))
            (else
              (goto _label_8))))))))

(event `Reset3`
  (goto _label_5 :!via `Reset`))

(event `Reset4`
  (goto _label_7 :!via `Reset`))

(fn `UserConstructionScript`)

(fn `VerificaError`
  (params (ID :type Integer))
  (returns (Liberado :type Boolean))
  (for _array_element (`/Game/Grid/BP_Generator.IDError` (`self.Grid`))
    (if (== _array_element ID)
      (return false)))
  (return true))