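; GM_Player is a game mode, by its name, that sets up audio mixing and can restore saved volume settings.
; BeginPlay and the construction script both set SFX_Master as the base sound mix and print a debug message if the GameSettings save is missing.
; Load_Save loads that slot and applies SoundVolumes by index as music, ambient and effects class overrides, but neither graph calls it.
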(event `self.ReceiveBeginPlay`
  (`GameplayStatics.SetBaseSoundMix` "/Game/Sounds/Classes/SFX_Master.SFX_Master")
  (bind _returnvalue (`GameplayStatics.DoesSaveGameExist` "GameSettings"))
  (if (not _returnvalue)
    (`KismetSystemLibrary.PrintString` "save inexistente")))

(fn `UserConstructionScript`
  (`GameplayStatics.SetBaseSoundMix` "/Game/Sounds/Classes/SFX_Master.SFX_Master")
  (bind _returnvalue (`GameplayStatics.DoesSaveGameExist` "GameSettings"))
  (if (not _returnvalue)
    (`KismetSystemLibrary.PrintString` "save inexistente")))