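; BP_GM, apparently a game mode, applies the player's saved audio volumes.
; Its Construction Script sets SFX_Master as the base sound mix, then runs the Load Save macro if a GameSettings save slot exists.
; The macro casts the save to GameSettings and maps its SoundVolumes array by index to music, ambient and effects sound class overrides.
; BeginPlay and Tick are empty, and debug prints report the save state.
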(event `self.ReceiveBeginPlay`)

(fn `UserConstructionScript`
  (`GameplayStatics.SetBaseSoundMix` "/Game/Sounds/Classes/SFX_Master.SFX_Master")
  (bind _returnvalue (`GameplayStatics.DoesSaveGameExist` "GameSettings"))
  (if _returnvalue
    (`self.Load Save`
      (:`Segue o baile`
        (`KismetSystemLibrary.PrintString` "Save gigante carregado")))
    (else
      (`KismetSystemLibrary.PrintString` "save inexistente"))))